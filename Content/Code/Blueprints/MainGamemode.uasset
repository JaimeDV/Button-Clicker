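; Main game mode for a pop-up window game that creates the main UI, health bar and dimming overlay, and opens the game-over level.
; While running, Tick uses a Delay to spawn pop-ups at random screen positions, with a plain one first, then random basic, inverse or rotating variants.
; Each spawn shortens the next delay until it hits a floor.
; Tick also raises music volume as the health bar empties.
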(event `StartGame`
  ;[1 1 1] Start Game
  (bind _returnvalue (`|CreateWidget` "/Game/Code/Widgets/HealthBar_Ui.HealthBar_Ui_C" null null))
  (set `self.healthBar Ui` _returnvalue)
  (bind _returnvalue_2 (`|CreateWidget` "/Game/Code/Widgets/DimmingUi.DimmingUi_C" null (`self.healthBar Ui`)))
  (bind _output_get (set `self.DimmingEffect` _returnvalue_2))
  (`UserWidget.AddToViewport` _output_get 200)
  (set `self.GameInit` true)
  (`UserWidget.AddToViewport` (`self.healthBar Ui`) 4)
  (set `/Game/Code/Widgets/MainUi.HealthBar Ui` (`self.healthBar Ui`) (`self.Main Ui`)))

(event `GameOver`
  ;[1 1 1] EndGame
  (set `self.GameInit` false)
  (`GameplayStatics.OpenLevelBySoftObjectPtr` "/Game/Levels/GameOver.GameOver"))

(event `self.ReceiveBeginPlay`
  ;[1 1 1] Variable init
  (bind _returnvalue (`|CreateWidget` "/Game/Code/Widgets/MainUi.MainUi_C" null (`self.healthBar Ui`)))
  (bind _output_get (set `self.Main Ui` _returnvalue))
  (`UserWidget.AddToViewport` _returnvalue 0)
  (`UserWidget.AddToViewport` _output_get 0))

(event `self.ReceiveTick`
  (params (DeltaSeconds :type "Float (single-precision)"))
  (bind _healthbar_ui (`self.healthBar Ui`))
  ;[1 1 1] PopUpSpawn behaviour
  (`/Engine/EditorBlueprintResources/StandardMacros.IsValid` _healthbar_ui
    (:`Is Valid`
      (bind _output_get (set `self.Sound Volume` (* (- 1.0 (`ProgressBar.Percent` (`/Game/Code/Widgets/HealthBar_Ui.HealthBar` _healthbar_ui))) 2.0))))
    (:`Is Not Valid`
      (set `self.Sound Volume` 0.2)))
  (if (== _output_get 0.0)
    (set `self.Sound Volume` 0.2))
  (`AudioComponent.SetVolumeMultiplier` (`self.MusicPlayer`) (`self.Sound Volume`))
  (if (`self.GameInit`)
    ;;[1 1 1] When started ignore timer
    (if (not (`self.First PopUp`))
      (`KismetSystemLibrary.Delay` (`self.nextWindow`)))
    ;;[1 1 1] Ask twice to avoid straglers
    (if (`self.GameInit`)
      (if (`self.First PopUp`)
        (set `self.First PopUp` false)
        (bind _returnvalue (`|CreateWidget` "/Game/Code/Widgets/PopUp.PopUp_C" null (`self.healthBar Ui`) :!label _label))
        (`self.Create Pop Up` _returnvalue)
        (else
          (switch `int` (`KismetMathLibrary.RandomIntegerInRange` 0 3)
            (:`Default`
              (goto _label))
            (:`0`
              (goto _label))
            (:`1`
              (goto _label))
            (:`2`
              (bind _returnvalue_2 (`|CreateWidget` "/Game/Code/Widgets/PopUp_Inverse.PopUp_Inverse_C" null (`self.healthBar Ui`)))
              (`self.Create Pop Up` _returnvalue_2))
            (:`3`
              (bind _returnvalue_3 (`|CreateWidget` "/Game/Code/Widgets/PopUp_Rotating.PopUp_Rotating_C" null (`self.healthBar Ui`)))
              (`self.Create Pop Up` _returnvalue_3)))))
      (bind _output_get_2 (set `self.nextWindow` (- (`self.nextWindow`) (`self.timerDecay`))))
      (if (<= _output_get_2 (`self.MinTimer`))
        (set `self.nextWindow` 0.2))
      (set `self.nextWindow` (`self.nextWindow`)))))

(fn `Create Pop Up`
  (params (popUpUi :type "UserWidget Object Reference"))
  (bind (_x _y) (`KismetMathLibrary.BreakVector2D` (`WidgetLayoutLibrary.GetViewportSize`)))
  (set `self.popUpUi` popUpUi)
  (`UserWidget.AddToViewport` (`self.popUpUi`) 0)
  (`UserWidget.SetPositionInViewport` (`self.popUpUi`) (0.0 0.0) true)
  (`UserWidget.SetAlignmentInViewport` (`self.popUpUi`) (`KismetMathLibrary.MakeVector2D` (/ (/ (* _x (`KismetMathLibrary.RandomFloatInRange` -5.1 1.0)) (`WidgetLayoutLibrary.GetViewportScale`)) 10000.0) (/ (/ (* _y (`KismetMathLibrary.RandomFloatInRange` -4.5 -0.6)) (`WidgetLayoutLibrary.GetViewportScale`)) 10000.0))))

(fn `UserConstructionScript`)